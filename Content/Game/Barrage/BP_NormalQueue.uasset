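; BP_NormalQueue is a short-lived worker actor that runs repeated, queued calls for the barrage system's BP_WebSocketServer.
; On BeginPlay it invokes the server function named by CallName, waits for Delay, then decrements that name's count in the server's NormalQueue map.
; While the count stays positive it spawns a copy of itself as the next iteration; otherwise it removes the entry, destroying itself either way.
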(event EventBeginPlay
  (bind _asbp_web_socket_server (Utilities|Casting|CastToBP_WebSocketServer (Variables|Default|GetActor)))
  (Variables|Default|SetAs%20BP%20Web%20Socket%20Server _asbp_web_socket_server)
  (Default|CallFunction (Variables|Default|GetAs%20BP%20Web%20Socket%20Server) (Variables|Default|GetCallName))
  (Utilities|FlowControl|Delay (Variables|Default|GetDelay))
  (Utilities|Map|Add (Variables|/Game/Game/Barrage/BP_WebSocketServer.BP_WebSocketServer_C|GetNormalQueue (Variables|Default|GetAs%20BP%20Web%20Socket%20Server)) (Variables|Default|GetCallName) (- (.Value (Utilities|Map|Find (Variables|/Game/Game/Barrage/BP_WebSocketServer.BP_WebSocketServer_C|GetNormalQueue (Variables|Default|GetAs%20BP%20Web%20Socket%20Server)) (Variables|Default|GetCallName))) 1))
  (if (> (.Value (Utilities|Map|Find (Variables|/Game/Game/Barrage/BP_WebSocketServer.BP_WebSocketServer_C|GetNormalQueue (Variables|Default|GetAs%20BP%20Web%20Socket%20Server)) (Variables|Default|GetCallName))) 0)
    (Game|SpawnActorfromClass "BP_NormalQueue_C" (Math|Transform|MakeTransform "0, 0, 0" "0, 0, 0" "1.000000,1.000000,1.000000") "Undefined" "MultiplyWithRoot" 0 (Variables|Default|GetAs%20BP%20Web%20Socket%20Server) (Variables|Default|GetCallName) (Variables|Default|GetDelay) 0)
    (Actor|DestroyActor)
    (else
      (Utilities|Map|Remove (Variables|/Game/Game/Barrage/BP_WebSocketServer.BP_WebSocketServer_C|GetNormalQueue (Variables|Default|GetAs%20BP%20Web%20Socket%20Server)) (Variables|Default|GetCallName))
      (Actor|DestroyActor))))

(event Collision|EventActorBeginOverlap
  (params (OtherActor :type Actor%20Object%20Reference)))

(event EventTick
  (params (DeltaSeconds :type Float%20%28single-precision%29)))

(fn ConstructionScript)