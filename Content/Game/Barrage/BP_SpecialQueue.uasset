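; BP_SpecialQueue is a self-respawning actor that works through one named entry in the WebSocket server's SpecialQueue count map, apparently for barrage-triggered special effects.
; Without a matching video, it calls the named functions on the server, waits, then decrements the count.
; It respawns itself while count remains, otherwise removes the entry, and destroys itself either way.
; Video playback looks disconnected: a found video halts BeginPlay, and the destroy-bound resume is never wired here.
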(event Custom|Start
  (params (DestroyedActor :type Actor%20Object%20Reference))
  (bind _asbp_web_socket_server (Utilities|Casting|CastToBP_WebSocketServer (Variables|Default|GetActor)))
  (Variables|Default|SetAs%20BP%20Web%20Socket%20Server _asbp_web_socket_server)
  (for _array_element (Variables|Default|GetCallName)
    (Default|CallFunction (Variables|Default|GetAs%20BP%20Web%20Socket%20Server) _array_element))
  (Utilities|FlowControl|Delay (Variables|Default|GetDelay))
  (Utilities|Map|Add (Variables|/Game/Game/Barrage/BP_WebSocketServer.BP_WebSocketServer_C|GetSpecialQueue (Variables|Default|GetAs%20BP%20Web%20Socket%20Server)) (Variables|Default|GetSettingName) (- (.Value (Utilities|Map|Find (Variables|/Game/Game/Barrage/BP_WebSocketServer.BP_WebSocketServer_C|GetSpecialQueue (Variables|Default|GetAs%20BP%20Web%20Socket%20Server)) (Variables|Default|GetSettingName))) 1))
  (if (> (.Value (Utilities|Map|Find (Variables|/Game/Game/Barrage/BP_WebSocketServer.BP_WebSocketServer_C|GetSpecialQueue (Variables|Default|GetAs%20BP%20Web%20Socket%20Server)) (Variables|Default|GetSettingName))) 0)
    (Game|SpawnActorfromClass "BP_SpecialQueue_C" (Math|Transform|MakeTransform "0, 0, 0" "0, 0, 0" "1.000000,1.000000,1.000000") "Undefined" "MultiplyWithRoot" 0 (Variables|Default|GetAs%20BP%20Web%20Socket%20Server) (Variables|Default|GetSettingName) (Variables|Default|GetCallName) (Variables|Default|GetDelay) (Variables|Default|GetVideoName) 0)
    (Actor|DestroyActor)
    (else
      (Utilities|Map|Remove (Variables|/Game/Game/Barrage/BP_WebSocketServer.BP_WebSocketServer_C|GetSpecialQueue (Variables|Default|GetAs%20BP%20Web%20Socket%20Server)) (Variables|Default|GetSettingName))
      (Actor|DestroyActor))))

(event EventBeginPlay
  (CallFunction|InitManager)
  (for _array_element (Variables|Default|GetBoxVideo)
    (if (Utilities|String|Contains (Utilities|GetObjectName _array_element) (Variables|Default|GetVideoName))
      (Variables|Default|SetCurrentVideo _array_element)))
  (Utilities|IsValid (Variables|Default|GetCurrentVideo)
    (:Is%20Not%20Valid
      (bind _asbp_web_socket_server (Utilities|Casting|CastToBP_WebSocketServer (Variables|Default|GetActor)))
      (Variables|Default|SetAs%20BP%20Web%20Socket%20Server _asbp_web_socket_server)
      (for _array_element_2 (Variables|Default|GetCallName)
        (Default|CallFunction (Variables|Default|GetAs%20BP%20Web%20Socket%20Server) _array_element_2))
      (Utilities|FlowControl|Delay (Variables|Default|GetDelay))
      (Utilities|Map|Add (Variables|/Game/Game/Barrage/BP_WebSocketServer.BP_WebSocketServer_C|GetSpecialQueue (Variables|Default|GetAs%20BP%20Web%20Socket%20Server)) (Variables|Default|GetSettingName) (- (.Value (Utilities|Map|Find (Variables|/Game/Game/Barrage/BP_WebSocketServer.BP_WebSocketServer_C|GetSpecialQueue (Variables|Default|GetAs%20BP%20Web%20Socket%20Server)) (Variables|Default|GetSettingName))) 1))
      (if (> (.Value (Utilities|Map|Find (Variables|/Game/Game/Barrage/BP_WebSocketServer.BP_WebSocketServer_C|GetSpecialQueue (Variables|Default|GetAs%20BP%20Web%20Socket%20Server)) (Variables|Default|GetSettingName))) 0)
        (Game|SpawnActorfromClass "BP_SpecialQueue_C" (Math|Transform|MakeTransform "0, 0, 0" "0, 0, 0" "1.000000,1.000000,1.000000") "Undefined" "MultiplyWithRoot" 0 (Variables|Default|GetAs%20BP%20Web%20Socket%20Server) (Variables|Default|GetSettingName) (Variables|Default|GetCallName) (Variables|Default|GetDelay) (Variables|Default|GetVideoName) 0)
        (Actor|DestroyActor)
        (else
          (Utilities|Map|Remove (Variables|/Game/Game/Barrage/BP_WebSocketServer.BP_WebSocketServer_C|GetSpecialQueue (Variables|Default|GetAs%20BP%20Web%20Socket%20Server)) (Variables|Default|GetSettingName))
          (Actor|DestroyActor))))))

(event Collision|EventActorBeginOverlap
  (params (OtherActor :type Actor%20Object%20Reference)))

(event EventTick
  (params (DeltaSeconds :type Float%20%28single-precision%29)))

(fn ConstructionScript)

(fn InitManager
  (bind _returnvalue (Actor|GetActorOfClass 0))
  (Utilities|IsValid _returnvalue
    (:Is%20Valid
      (Variables|Default|SetVideoManager _returnvalue))))