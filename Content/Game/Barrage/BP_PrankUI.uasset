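; BP_PrankUI is an actor that toggles the WBP_Prank widget on screen with the Tab key.
; It enables player input on BeginPlay, and each Tab press flips IsShow through ChangeUI.
; Showing creates a fresh widget at a high Z-order, displays the cursor and switches to Game and UI input.
; Hiding removes the widget, hides the cursor and restores game-only input.
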(event EventBeginPlay
  (Input|EnableInput (Game|GetPlayerController 0)))

(event Collision|EventActorBeginOverlap
  (params (OtherActor :type Actor%20Object%20Reference)))

(event EventTick
  (params (DeltaSeconds :type Float%20%28single-precision%29)))

(event Input|KeyboardEvents|Tab
  (params (Key :type Key%20Structure :default "None"))
  (:Pressed
    (CallFunction|ChangeUI)))

(fn ConstructionScript)

(fn ChangeUI
  (bind _returnvalue (Game|GetPlayerController 0))
  (bind _returnvalue_2 (Game|GetPlayerController 0))
  (bind _output_get (Variables|Default|SetIsShow (not (Variables|Default|GetIsShow))))
  (if _output_get
    (bind _returnvalue_3 (UserInterface|CreateWidget "/Game/Game/Barrage/UI/WBP_Prank.WBP_Prank_C"))
    (bind _output_get_2 (Variables|Default|SetWBP_Prank _returnvalue_3))
    (UserInterface|Viewport|AddtoViewport _output_get_2 500)
    (Variables|/Script/Engine.PlayerController|SetbShowMouseCursor _returnvalue true)
    (Input|SetInputModeGameandUI _returnvalue_2 (Variables|Default|GetWBP_Prank) "DoNotLock" true false)
    (else
      (Widget|RemovefromParent (Variables|Default|GetWBP_Prank))
      (Variables|/Script/Engine.PlayerController|SetbShowMouseCursor _returnvalue false)
      (Input|SetInputModeGameOnly _returnvalue_2 false))))